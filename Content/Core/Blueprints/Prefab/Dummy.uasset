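; Dummy is a target actor prefab that displays its health and reacts to melee hits.
; Every tick it writes the health component's current health, truncated to an integer, to a text element.
; MeleeHit applies damage to itself with a fixed negative base value, and the health component's OnDeath event destroys the actor.
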(event OnDeath(C_Health_Component)
  (Actor|DestroyActor))

(event EventTick
  (params (DeltaSeconds :type Float%20%28single-precision%29))
  (Rendering|Components|TextRender|SetText (Variables|Default|GetHeath) (Utilities|Text|ToText(Integer) (Math|Float|Truncate (Variables|/Game/Core/Blueprints/Component/HealthComponent.HealthComponent_C|GetCurrent%20Health (Variables|Default|GetC_Health_Component))))))

(event Collision|EventActorBeginOverlap
  (params (OtherActor :type Actor%20Object%20Reference)))

(event EventMeleeHit
  (Game|Damage|ApplyDamage self -4e+01 0 0))

(event EventBeginPlay)

(fn ConstructionScript)