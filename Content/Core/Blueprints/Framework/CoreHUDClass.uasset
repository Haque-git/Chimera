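; Core HUD class that creates the main HUD and pause menu widgets and manages switching between game and menu focus.
; Menus live in a widget list, so toggling one collapses the others and sets input mode and cursor visibility.
; It caches CoreGameMode, pushes the initial time, then binds its time-update and round-end delegates to refresh the HUD timer and show the result.
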(event Custom|On%20Round%20End
  ;[0.1042 0.1042 0.1042] On Round End
  (Default|ShowResult (Variables|Default|GetMainHUD)))

(event Custom|Bind%20Round%20End
  ;[0.1042 0.1042 0.1042] On Round End
  (EventDispatchers|AssignOnRoundEnd (Variables|Components|GetGameMode) (delegate Custom|On%20Round%20End)))

(event Custom|On%20Time%20Update_Event
  (params (Min :type Integer) (Sec :type Integer))
  ;[0.1042 0.1042 0.1042] Bind Time
  (Default|UpdateTime (Variables|Default|GetMainHUD) Min Sec))

(event Custom|Bind%20Time%20Update
  ;[0.1042 0.1042 0.1042] Bind Time
  (EventDispatchers|AssignOnTimeUpdate (Variables|Components|GetGameMode) (delegate Custom|On%20Time%20Update_Event)))

(event EventBeginPlay
  ;[0.1042 0.1042 0.1042] Begin Play
  (Utilities|FlowControl|Sequence
    (:then_0
      ;[0.1042 0.1042 0.1042] Set Input Mode Game Only
      (Input|SetInputModeGameOnly (Game|GetPlayerController 0))
      (Utilities|FlowControl|Sequence
        (:then_0
          ;[0.1042 0.1042 0.1042] Game Menus
          ;;[0.1042 0.1042 0.1042] HUD
          (bind _returnvalue (UserInterface|CreateWidget "/Game/Core/UI/WBP_HUD.WBP_HUD_C" (Game|GetPlayerController 0)))
          (bind _output_get (Variables|Default|SetMainHUD _returnvalue))
          (UserInterface|Viewport|AddtoViewport _output_get 0))
        (:then_1
          ;;[0.1042 0.1042 0.1042] Pause Menu
          (bind _returnvalue_2 (UserInterface|CreateWidget "/Game/Core/UI/WBP_PauseMenu.WBP_PauseMenu_C" (Game|GetPlayerController 0)))
          (bind _output_get_2 (Variables|Default|SetPauseMenu _returnvalue_2))
          (Utilities|Array|Add (Variables|Widgets|GetGame%20Menu%20Widget%20List) _output_get_2))
        (:then_2
          ;;[0.1042 0.1042 0.1042] Add All To Viewport
          (for _array_element (Variables|Widgets|GetGame%20Menu%20Widget%20List)
            (UserInterface|Viewport|AddtoViewport _array_element 0)))))
    (:then_1
      ;[0.1042 0.1042 0.1042] References
      (|References)
      (|InitialUpdates))
    (:then_2
      ;[0.1042 0.1042 0.1042] Bind Events
      (CallFunction|BindTimeUpdate)
      (CallFunction|BindRoundEnd))))

(event Custom|Toggle%20Pause%20Menu
  ;[0.1042 0.1042 0.1042] Toggling Widgets
  (CallFunction|ToggleGameMenuWidget (Variables|Default|GetPauseMenu) true))

(fn ConstructionScript)

(fn ToggleGameMenuWidget
  (params (Target%20Widget :type User%20Widget%20Object%20Reference) (Show%20Cursor? :type Boolean))
  (Utilities|IsValid Target%20Widget
    (:Is%20Valid
      (Variables|Widgets|SetWidget%20To%20Focus Target%20Widget)
      (for _array_element (Variables|Widgets|GetGame%20Menu%20Widget%20List)
        (if (== (Variables|Widgets|GetWidget%20To%20Focus) _array_element)
          (if (Widget|IsVisible (Variables|Widgets|GetWidget%20To%20Focus))
            (CallFunction|FocusGame)
            (else
              (CallFunction|FocusWidget Show%20Cursor?)))
          (elif (Widget|IsVisible _array_element)
            (Widget|SetVisibility _array_element "Collapsed")))))))

(fn FocusGame
  (bind _returnvalue (Game|Player|GetOwningPlayerController))
  (Widget|SetVisibility (Variables|Widgets|GetWidget%20To%20Focus) "Collapsed")
  (Input|SetInputModeGameOnly _returnvalue)
  (Variables|/Script/Engine.PlayerController|SetbShowMouseCursor _returnvalue false))

(fn FocusWidget
  (params (Cursor :type Boolean))
  (bind _returnvalue (Game|Player|GetOwningPlayerController))
  (bind _widget_to_focus (Variables|Widgets|GetWidget%20To%20Focus))
  (Widget|SetVisibility _widget_to_focus "SelfHitTestInvisible")
  (Input|SetInputModeGameandUI _returnvalue _widget_to_focus "DoNotLock" true)
  (if Cursor
    (Variables|/Script/Engine.PlayerController|SetbShowMouseCursor _returnvalue true)))