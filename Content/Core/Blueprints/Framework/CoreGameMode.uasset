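; Game mode that runs a round countdown and signals when the round is over.
; On BeginPlay it splits the round time into minutes and seconds and starts a looping one-second timer.
; Each tick decrements the clock and broadcasts OnTimeUpdate through an event dispatcher.
; When the round-end check passes at zero, it broadcasts OnRoundEnd and clears the timer.
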(event Custom|Countdown%20Event
  ;[0.1042 0.1042 0.1042] Timer
  (Utilities|FlowControl|Sequence
    (:then_0
      ;;[0.1042 0.1042 0.1042] Calculate Time
      (|CalculateTime))
    (:then_1
      (Default|CallOnTimeUpdate (Variables|Private|GetMinutes) (Variables|Private|GetSeconds)))
    (:then_2
      (if (Utilities|CanCallRoundEnd)
        (Default|CallOnRoundEnd)
        (Utilities|Time|ClearandInvalidateTimerbyHandle (Variables|Default|GetTimer%20Handle))))))

(event Custom|Countdown
  ;[0.1042 0.1042 0.1042] Timer
  (bind _returnvalue (Utilities|Time|SetTimerbyEvent (delegate Custom|Countdown%20Event) 1.0 true))
  (Variables|Default|SetTimer%20Handle _returnvalue))

(event EventBeginPlay
  (Utilities|FlowControl|Sequence
    (:then_0
      ;[0.1042 0.1042 0.1042] Timer
      (|Timer))))

(fn ConstructionScript)

(fn SecondstoMinutes
  (bind _output_get (LocalVariables|SetSecondary%20Time (Variables|Default|GetRound%20Time%20%28s%29)))
  (LocalVariables|SetSeconds%28Local%29 (Math|Integer|%(Integer) _output_get 60))
  (LocalVariables|SetMinutes%28Local%29 (/ _output_get 60))
  (return (LocalVariables|GetSeconds%28Local%29) (LocalVariables|GetMinutes%28Local%29)))