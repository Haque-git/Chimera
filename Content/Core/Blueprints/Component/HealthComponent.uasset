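; Health component that tracks its owning actor's health and signals when it changes or runs out.
; On BeginPlay it binds to the owner's OnTakeAnyDamage event.
; Each hit adds the Damage value to CurrentHealth, so only negative values reduce it, and clamps the result between zero and MaxHealth.
; It then broadcasts OnHealthChange, followed by OnDeath whenever health is at zero.
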(event Custom|On%20Damage
  (params (DamagedActor :type Actor%20Object%20Reference) (Damage :type Float%20%28single-precision%29) (DamageType :type Damage%20Type%20Object%20Reference) (InstigatedBy :type Controller%20Object%20Reference) (DamageCauser :type Actor%20Object%20Reference))
  (bind _output_get (Variables|Health|SetCurrent%20Health (Math|Float|Clamp(Float) (+ (Variables|Health|GetCurrent%20Health) Damage) 0.0 (Variables|Health|GetMax%20Health))))
  (Default|CallOnHealthChange _output_get (Variables|Health|GetMax%20Health))
  ;[0.1042 0.1042 0.1042] Death
  (if (<= (Variables|Health|GetCurrent%20Health) 0.0)
    (Default|CallOnDeath)))

(event EventBeginPlay
  ;[0.1042 0.1042 0.1042] On Any Damage
  (EventDispatchers|BindEventtoOnTakeAnyDamage (Components|GetOwner) (delegate Custom|On%20Damage)))