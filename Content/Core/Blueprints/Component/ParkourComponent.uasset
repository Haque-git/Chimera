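; Parkour component for Core_character that adds ledge vaulting and strafe camera tilt.
; Each tick, a vertical trace ahead checks height, walkable slope and capsule clearance to cache a landing point.
; The Vault event starts a per-tick location lerp to that point without sweep, then resets the state.
; A looping timer at about 60 Hz eases controller roll by strafe input while moving, leveling it at low speed.
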(event Custom|Vault%20Tick
  ;[0.1042 0.1042 0.1042] Vault Tick
  (Utilities|MVaultingState
    (:Can%20Vault
      (bind (_result _end_location) (Vault|CanVault))
      (if _result
        (Variables|Vault|SetEnd%20Location _end_location)))
    (:Vaulting
      (Vault|Vaulting (Variables|Defaults|GetDelta%20Seconds)))))

(event Custom|Update%20Event
  ;[0.1042 0.05751 0.05751] Use Instead Tick!
  (Utilities|FlowControl|Sequence
    (:then_0
      (|CameraUpdate))))

(event Custom|Update
  ;[0.1042 0.05751 0.05751] Use Instead Tick!
  (Utilities|Time|SetTimerbyEvent (delegate Custom|Update%20Event) 0.0167 true))

(event Custom|Event%20Vault
  ;[0.1042 0.1042 0.1042] Vault Event
  (Variables|Vault|SetInitial%20Location (Transformation|GetActorLocation (Variables|Components|GetCharacter)))
  (Variables|Vault|SetAlpha 0.0)
  (Variables|Vault|SetVaulting%20State "NewEnumerator2"))

(event EventBeginPlay
  ;[0.1042 0.1042 0.1042] Begin Play
  (Utilities|FlowControl|Sequence
    (:then_0
      (|References))
    (:then_1
      (CallFunction|Update))))

(event EventTick
  (params (DeltaSeconds :type Float%20%28single-precision%29))
  ;[0.1042 0.04394 0.04394] Tick
  (Variables|Defaults|SetDelta%20Seconds DeltaSeconds)
  (CallFunction|VaultTick))

(fn CanVault
  (bind _vault_range (Variables|Vault|GetVault%20Range))
  (bind _character (Variables|Components|GetCharacter))
  (bind _character_2 (Variables|Components|GetCharacter))
  (bind _returnvalue (Transformation|GetActorLocation _character))
  (bind _returnvalue_2 (Transformation|GetActorForwardVector _character))
  (bind _capsulecomponent (Variables|/Script/Engine.Character|GetCapsuleComponent _character_2))
  (bind _returnvalue_3 (* _returnvalue_2 _vault_range))
  (bind _returnvalue_4 (Components|Capsule|GetScaledCapsuleHalfHeight _capsulecomponent))
  (bind _returnvalue_5 (+ _returnvalue _returnvalue_3))
  (if (Utilities|Enum|Equal(Enum) (Variables|Vault|GetVaulting%20State) "NewEnumerator2")
    (return false "0, 0, 0")
    (else
      (bind (_outhit _returnvalue_6) (Collision|LineTraceByChannel (+ _returnvalue_5 (Math|Vector|MakeVector 0.0 0.0 _returnvalue_4)) (- _returnvalue_5 (Math|Vector|MakeVector 0.0 0.0 _returnvalue_4)) "TraceTypeQuery1" false (Utilities|Array|MakeArray (Variables|Components|GetCharacter)) "None"))
      (if _returnvalue_6
        (bind (_result _end_location) (Vault|CanVaulttoHit (Variables|/Script/Engine.Character|GetCapsuleComponent (Variables|Components|GetCharacter)) _outhit))
        (return _result _end_location)
        (else
          (return false "0, 0, 0"))))))

(fn CanVaulttoHit
  (params (Capsul :type Capsule%20Component%20Object%20Reference) (Hit :type Hit%20Result%20Structure))
  (bind _returnvalue (Components|Capsule|GetScaledCapsuleHalfHeight Capsul))
  (bind _returnvalue_2 (Components|Capsule|GetScaledCapsuleRadius Capsul))
  (Utilities|FlowControl|Sequence
    (:then_0
      ;[0.04688 0.04688 0.04688] Checking for valid height
      (if (not (Math|Float|InRange(Float) (Math|Float|Absolute(Float) (- (.Z (Math|Vector|BreakVector (.location Hit))) (.Z (Math|Vector|BreakVector (.traceend Hit))))) (Variables|Vault|GetMinnimum%20Vault%20Height) (Variables|Vault|GetMaximum%20Vault%20Height)))
        (return false (LocalVariables|GetEnd%20Locaton))))
    (:then_1
      ;[0.04688 0.04688 0.04688] Cheking for valid slope
      (if (< (.Z (Math|Vector|BreakVector (.normal Hit))) (Class|CharacterMovementComponent|GetWalkableFloorZ (Variables|/Script/Engine.Character|GetCharacterMovement (Variables|Components|GetCharacter))))
        (return false (LocalVariables|GetEnd%20Locaton))))
    (:then_2
      ;[0.04688 0.04688 0.04688] Checking for collition
      (bind _output_get (LocalVariables|SetEnd%20Locaton (+ (.location Hit) (Math|Vector|MakeVector 0.0 0.0 _returnvalue))))
      (bind _result (Vault|CollisionTest (+ _output_get (Math|Vector|MakeVector 0.0 0.0 _returnvalue_2)) _returnvalue_2 _returnvalue false))
      (if _result
        (return false (LocalVariables|GetEnd%20Locaton))))
    (:then_3
      (return true (LocalVariables|GetEnd%20Locaton)))))

(fn CollisionTest
  (params (Location :type Vector) (Radious :type Float%20%28single-precision%29) (Height :type Float%20%28single-precision%29) (Draw%20debug :type Boolean))
  (Utilities|FlowControl|Sequence
    (:then_0
      (if Draw%20debug
        (Rendering|Debug|DrawDebugCapsule Location Height Radious "0, 0, 0" "(R=1.000000,G=1.000000,B=1.000000,A=1.000000)" 0.0 0.0)))
    (:then_1
      (bind _returnvalue (Collision|CapsuleOverlapActors Location Radious Height (Utilities|Array|MakeArray "ObjectTypeQuery1" "ObjectTypeQuery2" "ObjectTypeQuery4" "ObjectTypeQuery5" "ObjectTypeQuery6") "/Script/Engine.Actor" (Utilities|Array|MakeArray (Variables|Components|GetCharacter))))
      (return _returnvalue))))

(fn Vaulting
  (params (Delta%20Seconds :type Float%20%28single-precision%29))
  (Variables|Vault|SetAlpha (Math|Float|Clamp(Float) (+ (* Delta%20Seconds (Variables|Vault|GetVaulting%20Speed)) (Variables|Vault|GetAlpha))))
  (Transformation|SetActorLocation (Variables|Components|GetCharacter) (Math|Vector|Lerp(Vector) (Variables|Vault|GetInitial%20Location) (Variables|Vault|GetEnd%20Location) (Variables|Vault|GetAlpha)) false false)
  (if (>= (Variables|Vault|GetAlpha) 1.0)
    (Variables|Vault|SetVaulting%20State "NewEnumerator0")))

(fn GetSpeed
  (return (Math|Vector|VectorLength (Variables|/Script/Engine.MovementComponent|GetVelocity (Variables|Components|GetMovement)))))

(fn CameraTilt
  (params (Target%20X%20%28Roll%29 :type Float%20%28single-precision%29))
  (bind _character (Variables|Components|GetCharacter))
  (bind _returnvalue (Pawn|GetController _character))
  (bind _returnvalue_2 (Pawn|GetControlRotation _returnvalue :!class /Script/Engine.Controller))
  (bind (_roll _pitch _yaw) (Math|Rotator|BreakRotator _returnvalue_2))
  (Pawn|SetControlRotation (Pawn|GetController (Variables|Components|GetCharacter)) (Math|Interpolation|RInterpTo _returnvalue_2 (Math|Rotator|MakeRotator Target%20X%20%28Roll%29 _pitch _yaw) (Utilities|Time|GetWorldDeltaSeconds) 5.0)))

(fn HorizontalCameraTilt
  (params (Left :type Float%20%28single-precision%29) (Right :type Float%20%28single-precision%29))
  (if (<= (Movement|GetSpeed) 1e+02)
    (CallFunction|CameraTilt 0.0)
    (elif (< (Variables|/Game/Core/Blueprints/Core_character.Core_character_C|GetRigthAxisValue (Variables|Components|GetCharacter)) 0.0)
      (CallFunction|CameraTilt Left)
      (elif (> (Variables|/Game/Core/Blueprints/Core_character.Core_character_C|GetRigthAxisValue (Variables|Components|GetCharacter)) 0.0)
        (CallFunction|CameraTilt Right)))))

(fn DirectionalImpulse
  (params (Target :type Character%20Movement%20Component%20Object%20Reference) (Force :type Float%20%28single-precision%29))
  (Physics|AddImpulse Target (* (Pawn|Components|CharacterMovement|GetCurrentAcceleration (Variables|Components|GetMovement)) Force) false))

(fn GetAccelaration
  (return (Math|Vector|Normalize (Pawn|Components|CharacterMovement|GetCurrentAcceleration (Variables|/Script/Engine.Character|GetCharacterMovement (Variables|Components|GetCharacter))))))

(fn IsWalking
  (return (Pawn|Components|CharacterMovement|IsWalking (Variables|/Script/Engine.Character|GetCharacterMovement (Variables|Components|GetCharacter)))))